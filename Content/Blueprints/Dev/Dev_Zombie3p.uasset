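; Development third-person zombie Character that is driven directly by player input.
; Movement axes follow the controller's yaw, look axes feed controller pitch and yaw, and Jump triggers the standard character jump.
; The Attack input casts the mesh's anim instance to ABP_McVR_Zombie and plays the first zombie attack montage on it, with no hit or damage logic in the graph.
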(event `InputAxis|MoveForward`
  (params (AxisValue :type "Float (single-precision)"))
  ;[1 1 1] MovementInput
  (`self.AddMovementInput` (`KismetMathLibrary.GetForwardVector` (`KismetMathLibrary.MakeRotator` 0.0 0.0 (.yaw (`self.GetControlRotation`)))) AxisValue))

(event `InputAxis|MoveRight`
  (params (AxisValue :type "Float (single-precision)"))
  ;[1 1 1] MovementInput
  (`self.AddMovementInput` (`KismetMathLibrary.GetRightVector` (`KismetMathLibrary.MakeRotator` 0.0 0.0 (.yaw (`self.GetControlRotation`)))) AxisValue))

(event `InputAction|Attack`
  (params (Key :type "Key Structure"))
  ;[1 1 1] AttackInput
  (:`Pressed`
    (bind _asabp_mc_vr_zombie (cast `/Game/Models/Zombie/ABP_McVR_Zombie` (`SkeletalMeshComponent.GetAnimInstance` (`self.Mesh`))))
    (`AnimInstance.Montage_Play` _asabp_mc_vr_zombie "/Game/Models/Zombie/M_Zombie_Attack1.M_Zombie_Attack1" 1.0 "MontageLength" 0.0)))

(event `InputAxis|LookUp`
  (params (AxisValue :type "Float (single-precision)"))
  ;[1 1 1] LookInput
  (`self.AddControllerPitchInput` AxisValue))

(event `InputAxis|LookRight`
  (params (AxisValue :type "Float (single-precision)"))
  ;[1 1 1] LookInput
  (`self.AddControllerYawInput` AxisValue))

(event `InputAction|Jump`
  (params (Key :type "Key Structure"))
  (:`Pressed`
    (`self.Jump`)))

(fn `UserConstructionScript`)