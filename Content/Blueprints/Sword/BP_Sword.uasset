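; Sword actor that is picked up by a hand and damages BP_McVR_Zombie actors it overlaps.
; PickUp and Drop toggle physics, collision profile and attachment; pickup also notifies the GameManager.
; Tick derives a swing velocity from position change multiplied by delta time, and fast hits deal boosted damage with a crit sound.
; A DoOnce with a short delay throttles hits.
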(event `/Game/Blueprints/Sword/BPI_Interactable.Interact`)

(event `self.ReceiveBeginPlay`)

(event `self.ReceiveTick`
  (params (DeltaSeconds :type "Float (single-precision)"))
  (set `self.DeltaTime` DeltaSeconds)
  (`self.UpdateVelocity`))

(event `Event Pick Up`
  (params (Hand :type "SceneComponent Object Reference"))
  (bind _sm_sword (`self.SM_Sword`))
  ;[1 1 1] PickUp/Drop
  (set `self.PickedUp` true)
  (`PrimitiveComponent.SetSimulatePhysics` _sm_sword false)
  (`PrimitiveComponent.SetCollisionProfileName` _sm_sword "Weapon")
  (`self.K2_AttachToComponent` Hand "None" "SnapToTarget" "SnapToTarget" "SnapToTarget" false)
  (`/Game/Blueprints/BP_Game_Manager.Event_PickUp` (`self.Game Manager`)))

(event `Event Drop`
  (bind _sm_sword (`self.SM_Sword`))
  ;[1 1 1] PickUp/Drop
  (set `self.PickedUp` false)
  (`PrimitiveComponent.SetSimulatePhysics` _sm_sword true)
  (`PrimitiveComponent.SetCollisionProfileName` _sm_sword "PhysicsActor")
  (`self.K2_DetachFromActor` "KeepWorld" "KeepWorld" "KeepWorld"))

(event `Event Attack`
  (params (`Other Actor` :type "Actor Object Reference"))
  (bind _returnvalue (`self.K2_GetActorLocation`))
  (bind _returnvalue_2 (`GameplayStatics.GetPlayerPawn` 0))
  ;[1 1 1] Apply damage to zombie
  (if (>= (`KismetMathLibrary.VSize` (`self.Velocity`)) 0.09)
    (`GameplayStatics.ApplyDamage` `Other Actor` (* (`self.BaseDamage`) 1.5) null _returnvalue_2)
    (`GameplayStatics.PlaySoundAtLocation` "/Game/Sounds/SC_AttackCrit.SC_AttackCrit" _returnvalue)
    (else
      (`GameplayStatics.ApplyDamage` `Other Actor` (`self.BaseDamage`) null _returnvalue_2)
      (`GameplayStatics.PlaySoundAtLocation` "/Game/Sounds/SC_AttackStrong.SC_AttackStrong" _returnvalue))))

(event `self.ReceiveActorBeginOverlap`
  (params (OtherActor :type "Actor Object Reference"))
  ;[1 1 1] Apply damage to zombie
  (bind _asbp_mc_vr_zombie (cast `/Game/Blueprints/Zombie/BP_MCVR_Zombie` OtherActor))
  (`/Engine/EditorBlueprintResources/StandardMacros.DoOnce` false :!label _label
    (:`Completed`
      (`self.Event Attack` _asbp_mc_vr_zombie)
      (`KismetSystemLibrary.Delay` 0.2)
      (goto _label :!via `Reset`))))

(fn `UpdateVelocity`
  (returns (Velocity :type "Vector Structure"))
  (bind _returnvalue (`self.K2_GetActorLocation`))
  (bind _output_get (set `self.Velocity` (* (- (`self.LastKnownPosition`) _returnvalue) (`self.DeltaTime`))))
  (set `self.LastKnownPosition` _returnvalue)
  (return _output_get))

(fn `UserConstructionScript`)