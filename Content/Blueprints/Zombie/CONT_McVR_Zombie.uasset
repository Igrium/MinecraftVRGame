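; AI controller for the McVR zombie enemy that drives its behavior, attacks and death.
; On possess it caches the zombie's target, range and player capsule, runs the BT_McVR_Zombie_old behavior tree, writes Range to the blackboard and stores the player pawn.
; Attack forwards to the zombie pawn only while the player is alive.
; Die stops movement and tree logic, unpossesses and destroys the controller.
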(event `self.OnPossess`
  (params (PossessedPawn :type "Pawn Object Reference"))
  ;[1 1 1] Set up variables
  (bind _asbp_mc_vr_zombie (cast `/Game/Blueprints/Zombie/BP_MCVR_Zombie` PossessedPawn))
  (set `self.Zombie_Self` _asbp_mc_vr_zombie)
  (set `self.Target Actor` (`/Game/Blueprints/Zombie/BP_MCVR_Zombie.Target Actor` _asbp_mc_vr_zombie))
  (set `self.Range` (`/Game/Blueprints/Zombie/BP_MCVR_Zombie.Range` _asbp_mc_vr_zombie))
  (set `self.PlayerCapsule` (`/Game/Blueprints/Zombie/BP_MCVR_Zombie.PlayerCapsule` _asbp_mc_vr_zombie))
  (`self.RunBehaviorTree` "/Game/Blueprints/Zombie/BT_McVR_Zombie_old.BT_McVR_Zombie_old")
  (`BlackboardComponent.SetValueAsFloat` (`AIBlueprintHelperLibrary.GetBlackboard` null) "Range" (`self.Range`))
  (bind _asbp_mc_vr_default_pawn (cast `/Game/Blueprints/Player/BP_McVR_DefaultPawn` (`GameplayStatics.GetPlayerPawn` 0)))
  (set `self.Player_Pawn` _asbp_mc_vr_default_pawn))

(event `self.ReceiveTick`
  (params (DeltaSeconds :type "Float (single-precision)"))
  ;[1 1 1] Attack Logic
)

(event `Attack`
  ;[1 1 1] Attack Logic
  (if (`/Game/Blueprints/Player/BP_McVR_DefaultPawn.Alive` (`self.Player_Pawn`))
    (`/Game/Blueprints/Zombie/BP_MCVR_Zombie.Attack` (`self.Zombie_Self`) (`self.PlayerCapsule`))))

(event `Event Die`
  ;[1 1 1] Death Logic
  (`self.StopMovement`)
  (`BrainComponent.StopLogic` (`self.BrainComponent`) "")
  (`self.UnPossess`)
  (`self.K2_DestroyActor`))

(fn `UserConstructionScript`)