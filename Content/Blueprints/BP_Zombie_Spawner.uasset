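; BP_Zombie_Spawner is an actor that spawns an instance of a configurable class, by its name a zombie, at its own transform.
; A Spawn event creates the actor, adjusting for collisions but always spawning, then copies the spawner's range, hit range and fallback target onto it.
; It then plays its audio component unless the spawner is muted.
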(event `Event Spawn`
  (bind _returnvalue (`|SpawnActorFromClass` (`self.Class to Spawn`) (`self.GetTransform`) "AdjustIfPossibleButAlwaysSpawn" "OverrideRootScale" null 100.0 null))
  (set `/Game/Blueprints/Zombie/BP_MCVR_Zombie.Range` (`self.Range`) _returnvalue)
  (set `/Game/Blueprints/Zombie/BP_MCVR_Zombie.HitRange` (`self.HitRange`) _returnvalue)
  (set `/Game/Blueprints/Zombie/BP_MCVR_Zombie.Fallback Target Actor` (`self.Fallback Target Actor`) _returnvalue)
  (if (not (`self.Mute`))
    (`AudioComponent.Play` (`self.Audio`) 0.0)))

(fn `UserConstructionScript`)