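; BP_Sword_Respawnable is a placeable sword spawn point that creates a sword actor at its own transform.
; When StartSpawned is set it spawns on BeginPlay through the EventSpawn event.
; EventSpawn spawns SwordClass with the first player pawn as Instigator, adjusting for collisions, then passes its BaseDamage and GameManager to the new sword.
; No respawn trigger or timer is defined inside this Blueprint.
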(event `self.ReceiveBeginPlay`
  (if (`self.Start Spawned`)
    (`self.EventSpawn`)))

(event `EventSpawn`
  (bind _returnvalue (`|SpawnActorFromClass` (`self.SwordClass`) (`self.GetTransform`) "AdjustIfPossibleButAlwaysSpawn" "OverrideRootScale" null (`GameplayStatics.GetPlayerPawn` 0)))
  (set `/Game/Blueprints/Sword/BP_Sword.BaseDamage` (`self.BaseDamage`) _returnvalue)
  (set `/Game/Blueprints/Sword/BP_Sword.Game Manager` (`self.Game Manager`) _returnvalue))

(fn `UserConstructionScript`)