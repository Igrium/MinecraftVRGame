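; BP_Game_Manager runs zombie spawning for the VR game, starting the first time the sword pickup event fires.
; A self-rescheduling timer triggers spawners, shortening its interval each time down to about a minimum, so pressure ramps up.
; The first spawn uses FirstSpawnLocation, or a random pick if unset, and later spawns pick randomly from ZombieSpawners.
; It relays start and player-death events through dispatchers, and Stop halts timer rescheduling.
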(event `self.ReceiveBeginPlay`
  (bind _asbp_mc_vr_default_pawn (cast `/Game/Blueprints/Player/BP_McVR_DefaultPawn` (`GameplayStatics.GetPlayerPawn` 0)))
  (set `self.PlayerPawn` _asbp_mc_vr_default_pawn)
  (set `self.TimeBetweenSpawns` (`self.InitialTimeBetweenSpawns`))
  (add `/Game/Blueprints/Player/BP_McVR_DefaultPawn.Die` (`self.PlayerPawn`) (delegate `Event Die`))
  (if (not (`KismetSystemLibrary.IsValid` (`self.First Spawn Location`)))
    (set `self.First Spawn Location` (`self.GetRandomSpawnLocation`))))

(event `Event Die`
  (`self.EventDie`))

(event `Event_PickUp`
  ;[1 1 1] Sword Picked Up
  (`/Engine/EditorBlueprintResources/StandardMacros.DoOnce` false
    (:`Completed`
      (`self.Event Start`))))

(event `Event Start`
  ;[1 1 1] Start Spawning
  (set `self.TimerOn` true)
  (`self.Start Timer`)
  (`self.EventStart`))

(event `Event Stop`
  ;[1 1 1] Stop Spawning
  (set `self.TimerOn` false))

(event `Event RandomSpawn`
  ;[1 1 1] Random Spawn
  (if (`self.FirstSpawn`)
    (`/Game/Blueprints/BP_Zombie_Spawner.Event Spawn` (`self.First Spawn Location`))
    (else
      (`/Game/Blueprints/BP_Zombie_Spawner.Event Spawn` (`self.GetRandomSpawnLocation`))))
  (set `self.FirstSpawn` false))

(event `Start Timer`
  (bind _timebetweenspawns (`self.TimeBetweenSpawns`))
  ;[1 1 1] Start Timer
  (`self.Event RandomSpawn`)
  (if (>= _timebetweenspawns (`self.MinTimeBetweenSpawns`))
    (bind _output_get (set `self.TimeBetweenSpawns` (- _timebetweenspawns (`self.TimeRemovalPerSpawn`)))))
  (if (`self.TimerOn`)
    (`KismetSystemLibrary.K2_SetTimer` null "Start Timer" _output_get)))

(fn `GetRandomSpawnLocation`
  (returns (`Return Value` :type "/Game/Blueprints/BP_Zombie_Spawner Object Reference"))
  (bind _zombie_spawners (`self.Zombie Spawners`))
  (return (`|GetArrayItem` _zombie_spawners (`KismetMathLibrary.RandomIntegerInRange` 0 (- (`KismetArrayLibrary.Array_Length` _zombie_spawners) 1)))))

(fn `UserConstructionScript`)