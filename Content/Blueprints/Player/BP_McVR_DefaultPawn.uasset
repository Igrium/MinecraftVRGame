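; VR player pawn with floor tracking that lets the player grab and drop swords in either hand and handles damage and death.
; Tick moves the player capsule under the VR camera while alive, and hand trigger overlaps drive sword pickup, hiding that hand's mesh.
; Damage lowers health and flashes the camera tint, lasting longer at lower health.
; Death drops both swords, enables right-hand widget pointing and stops the survival timer started by the GameManager event.
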(event `self.ReceiveBeginPlay`
  (`HeadMountedDisplayFunctionLibrary.SetTrackingOrigin` "Floor")
  (set `PlayerController.bShowMouseCursor` true (`GameplayStatics.GetPlayerController` 0))
  (add `/Game/Blueprints/BP_Game_Manager.EventStart` (`self.GameManager`) (delegate `EventStart`)))

(event `EventStart`
  (`self.StartTimer`))

(event `self.ReceiveTick`
  (params (DeltaSeconds :type "Float (single-precision)"))
  (bind _returnvalue (`KismetMathLibrary.MakeVector` (.x (`SceneComponent.K2_GetComponentLocation` (`self.VRCamera`))) (.y (`SceneComponent.K2_GetComponentLocation` (`self.VRCamera`))) (- (.z (`SceneComponent.K2_GetComponentLocation` (`self.VRCamera`))) 80.0)))
  ;[0 0 0] Update Capsule Location
  (if (`self.Alive`)
    (`SceneComponent.K2_SetWorldLocation` (`self.PlayerCapsule`) _returnvalue false true)
    (set `self.PlayerWorldLocation` _returnvalue)))

(event `InputAction|ClickR`
  (params (Key :type "Key Structure"))
  (bind _widgetinteractionr (`self.WidgetInteractionR`))
  ;[0 0 0] Menu Interaction
  (:`Pressed`
    (if (`self.WidgetEnabled`)
      (`WidgetInteractionComponent.PressPointerKey` _widgetinteractionr "LeftMouseButton")))
  (:`Released`
    (`WidgetInteractionComponent.ReleasePointerKey` _widgetinteractionr "LeftMouseButton")))

(event `InputAction|GrabRight`
  (params (Key :type "Key Structure"))
  ;[0 0 0] Sword Logic
  (:`Pressed`
    (if (`self.Alive`)
      (if (`self.HoldingR`)
        (`self.DropR`)
        (else
          (`self.PickUpR`))))))

(event `InputAction|GrabLeft`
  (params (Key :type "Key Structure"))
  ;[0 0 0] Sword Logic
  (:`Pressed`
    (if (`self.Alive`)
      (if (`self.HoldingL`)
        (`self.DropL`)
        (else
          (`self.PickUpL`))))))

(event `self.ReceiveAnyDamage`
  (params (Damage :type "Float (single-precision)") (DamageType :type "DamageType Object Reference") (InstigatedBy :type "Controller Object Reference") (DamageCauser :type "Actor Object Reference"))
  ;[0 0 0] Damage Handling
  (bind _output_get (set `self.Health` (- (`self.Health`) Damage)))
  (`GameplayStatics.PlaySound2D` "/Game/Sounds/SC_PlayerHurt.SC_PlayerHurt")
  (if (<= _output_get 0.0)
    (`self.EventDie`)
    (else
      ;;[0 0 0] Flash Red
      (set `CameraComponent.PostProcessSettings` (make `PostProcessSettings` :`SceneColorTint` (`self.CameraTint`)) (`self.VRCamera`))
      (`KismetSystemLibrary.Delay` (* (/ 2.0 (`self.Health`)) 2.0))
      (set `CameraComponent.PostProcessSettings` (make `PostProcessSettings`) (`self.VRCamera`)))))

(event `EventDie`
  ;[0 0 0] Death
  (`self.Die`)
  (set `CameraComponent.PostProcessSettings` (make `PostProcessSettings` :`SceneColorTint` (`self.CameraTint`)) (`self.VRCamera`))
  (`self.DropL`)
  (`self.DropR`)
  (set `self.Alive` false)
  (set `self.WidgetEnabled` true)
  (`self.UpdateWidgetInteraction`)
  (`self.StopTimer`))

(event `UpdateTimer`
  ;[0 0 0] Update Timer
  (bind _output_get (set `self.Seconds` (+ (`self.Seconds`) 1)))
  (if (>= _output_get 60)
    (set `self.Seconds` 0)
    (set `self.Minutes` (+ (`self.Minutes`) 1))))

(event `StartTimer`
  ;[0 0 0] Timer
  (bind _returnvalue (`KismetSystemLibrary.K2_SetTimer` null "UpdateTimer" 1.0 true))
  (set `self.TimerHandle` _returnvalue))

(event `StopTimer`
  ;[0 0 0] Timer
  (`KismetSystemLibrary.K2_ClearAndInvalidateTimerHandle` (`self.TimerHandle`)))

(fn `DropL`
  (if (`self.HoldingL`)
    (set `self.HoldingL` false)
    (`/Game/Blueprints/Sword/BP_Sword.Event Drop` (`self.SwordL`))
    (`SceneComponent.SetVisibility` (`self.SM_Left`) true false)))

(fn `DropR`
  (if (`self.HoldingR`)
    (set `self.HoldingR` false)
    (`/Game/Blueprints/Sword/BP_Sword.Event Drop` (`self.SwordR`))
    (`SceneComponent.SetVisibility` (`self.SM_Right`) true false)))

(fn `PickUpL`
  (bind _sm_left (`self.SM_Left`))
  (bind _asbp_sword (cast `/Game/Blueprints/Sword/BP_Sword` (`|GetArrayItem` (`PrimitiveComponent.GetOverlappingActors` (`self.Trigger_Left`) "/Game/Blueprints/Sword/BP_Sword.BP_Sword_C"))))
  (bind _pickedup (`/Game/Blueprints/Sword/BP_Sword.PickedUp` _asbp_sword))
  (if _pickedup
    (`self.DropR`))
  (if _pickedup
    _
    (elif (`/Game/Blueprints/Sword/BP_Sword.CanHold` _asbp_sword)
      (set `self.HoldingL` true)
      (`/Game/Blueprints/Sword/BP_Sword.Event Pick Up` _asbp_sword _sm_left)
      (set `self.SwordL` _asbp_sword)
      (`SceneComponent.SetVisibility` _sm_left false false))))

(fn `PickUpR`
  (bind _sm_right (`self.SM_Right`))
  (bind _asbp_sword (cast `/Game/Blueprints/Sword/BP_Sword` (`|GetArrayItem` (`PrimitiveComponent.GetOverlappingActors` (`self.Trigger_Right`) "/Game/Blueprints/Sword/BP_Sword.BP_Sword_C"))))
  (bind _pickedup (`/Game/Blueprints/Sword/BP_Sword.PickedUp` _asbp_sword))
  (if _pickedup
    (`self.DropL`))
  (if _pickedup
    _
    (elif (`/Game/Blueprints/Sword/BP_Sword.CanHold` _asbp_sword)
      (set `self.HoldingR` true)
      (`/Game/Blueprints/Sword/BP_Sword.Event Pick Up` _asbp_sword _sm_right)
      (set `self.SwordR` _asbp_sword)
      (`SceneComponent.SetVisibility` _sm_right false false))))

(fn `UpdateWidgetInteraction`
  (set `WidgetInteractionComponent.bShowDebug` (`self.WidgetEnabled`) (`self.WidgetInteractionR`)))

(fn `UserConstructionScript`)